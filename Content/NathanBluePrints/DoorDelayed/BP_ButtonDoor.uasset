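; BP_ButtonDoor is an interactable button that opens a linked door for a limited time.
; Interact toggles MyDoor through OpenCloseDoor, waits Duration with a retriggerable delay, then toggles it again.
; An IsActive flag ignores further presses until the cycle finishes, so the delay is never restarted.
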(event `self.Interact`
  (if (not (`self.isActive`))
    (`/Game/NathanBluePrints/DoorDelayed/BP_DoorDelayed.OpenCloseDoor` (`self.myDoor`))
    (set `self.isActive` true)
    (`KismetSystemLibrary.RetriggerableDelay` (`self.duration`))
    (`/Game/NathanBluePrints/DoorDelayed/BP_DoorDelayed.OpenCloseDoor` (`self.myDoor`))
    (set `self.isActive` false)))

(fn `UserConstructionScript`
  (`parent.UserConstructionScript`))