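; BP_DoorDelayed is a door Actor that snaps its Pivot between two rotations based on MyButton's IsActive state.
; BeginPlay stores the actor's forward vector as StartRotation.
; OpenCloseDoor applies that direction as relative rotation when active, otherwise adds 45 to its Y component before converting.
; The offset is vector math rather than a 45-degree yaw, and no delay or interpolation is present.
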(event `self.ReceiveBeginPlay`
  (set `self.startRotation` (`KismetMathLibrary.Conv_RotatorToVector` (`self.K2_GetActorRotation`))))

(event `OpenCloseDoor`
  (if (`/Game/NathanBluePrints/DoorDelayed/BP_ButtonDoor.isActive` (`self.myButton`))
    (`SceneComponent.K2_SetRelativeRotation` (`self.Pivot`) (`KismetMathLibrary.Conv_VectorToRotator` (`self.startRotation`)) false false)
    (else
      (`SceneComponent.K2_SetRelativeRotation` (`self.Pivot`) (`KismetMathLibrary.Conv_VectorToRotator` (+ (`self.startRotation`) (0.0 45.0 0.0))) false false))))

(fn `UserConstructionScript`)