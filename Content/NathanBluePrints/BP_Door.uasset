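; BP_Door is a door that opens once when its Interact event fires, with no logic to close it.
; BeginPlay stores the actor's world forward vector as StartRotation.
; Interact sets IsOpen and instantly snaps Pivot's relative rotation, with no animation.
; The rotation comes from adding a large Y offset to that unit vector, so it points near 90 degrees yaw rather than turning by a set angle.
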(event `self.ReceiveBeginPlay`
  (set `self.startRotation` (`KismetMathLibrary.Conv_RotatorToVector` (`self.K2_GetActorRotation`))))

(event `self.Interact`
  (if (not (`self.isOpen`))
    (set `self.isOpen` true)
    (`SceneComponent.K2_SetRelativeRotation` (`self.Pivot`) (`KismetMathLibrary.Conv_VectorToRotator` (+ (`self.startRotation`) (0.0 45.0 0.0))) false false)))

(fn `UserConstructionScript`
  (`parent.UserConstructionScript`))