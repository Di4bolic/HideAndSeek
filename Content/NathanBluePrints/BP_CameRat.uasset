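; BP_CameRat is a surveillance camera that alerts a Boss when its PawnSensing spots the FirstPersonCharacter.
; If CameraTurn is set, Tick rotates it in yaw at Speed; with CameraClamp, it reverses Speed on reaching Min or Max offsets from its starting yaw.
; On a sighting, it sets itself as the Boss's ActualTarget and raises GoToTarget, unless that flag is already set.
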(event `self.ReceiveBeginPlay`
  (set `self.startTransform` (`self.GetTransform`)))

(event `self.ReceiveTick`
  (params (DeltaSeconds :type "Float (single-precision)"))
  (set `self.deltaSec` DeltaSeconds)
  (if (`self.cameraTurn`)
    (`self.K2_SetActorTransform` (`KismetMathLibrary.MakeTransform` (`self.K2_GetActorLocation`) (`KismetMathLibrary.MakeRotator` 0.0 0.0 (+ (* (`self.deltaSec`) (`self.speed`)) (.yaw (`self.K2_GetActorRotation`))))))
    (if (`self.CameraClamp`)
      (if (or (<= (.yaw (`self.K2_GetActorRotation`)) (+ (.yaw (.rotation (`self.startTransform`))) (`self.min`))) (>= (.yaw (`self.K2_GetActorRotation`)) (+ (.yaw (.rotation (`self.startTransform`))) (`self.max`))))
        (set `self.speed` (* -1 (`self.speed`)))))))

(event `self.PawnSensing.OnSeePawn`
  (params (Pawn :type "Pawn Object Reference"))
  (bind _boss (`self.boss`))
  (cast `/Game/FirstPersonBP/Blueprints/FirstPersonCharacter` Pawn)
  (if (not (`/Game/NathanBluePrints/AI_RatBoss.goToTarget` (`self.boss`)))
    (set `/Game/NathanBluePrints/AI_RatBoss.goToTarget` true _boss)
    (set `/Game/NathanBluePrints/AI_RatBoss.actualTarget` self _boss)))

(fn `UserConstructionScript`)