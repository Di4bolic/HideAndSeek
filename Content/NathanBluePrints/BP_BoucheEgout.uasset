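; BP_BoucheEgout is a manhole (sewer opening) that acts as a hiding spot for the player.
; On Interact it flags the player controller as hidden and teleports the pawn 100 units below the manhole's location.
; It then locks the FirstPersonCharacter's movement through CantMove.
; The graph has no exit logic, and a node disabling gravity on the character mesh is left unconnected.
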(event `self.Interact`
  (bind _asbp_my_player_controller (cast `/Game/EthanBluePrints/BP_MyPlayerController` (`GameplayStatics.GetPlayerController` 0)))
  (set `/Game/EthanBluePrints/BP_MyPlayerController.isHide` true _asbp_my_player_controller)
  (`self.K2_SetActorLocation` (`GameplayStatics.GetPlayerPawn` 0) (- (`self.K2_GetActorLocation` self) (0.0 0.0 100.0)) false true)
  (bind _asfirst_person_character (cast `/Game/FirstPersonBP/Blueprints/FirstPersonCharacter` (`GameplayStatics.GetPlayerCharacter` 0)))
  (set `/Game/FirstPersonBP/Blueprints/FirstPersonCharacter.cantMove` true _asfirst_person_character))

(fn `UserConstructionScript`
  (`parent.UserConstructionScript`))