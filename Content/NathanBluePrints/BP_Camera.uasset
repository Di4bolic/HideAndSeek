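; BP_Camera is a rotating watch camera that respawns the FirstPersonCharacter when its PawnSensing component sees it.
; Tick turns the actor in yaw at Speed while CameraTurn is set, zeroing pitch and roll and resetting scale to one.
; With CameraClamp also set, Speed flips sign whenever yaw reaches the Min or Max offset from the starting yaw, producing a back-and-forth sweep.
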(event `self.ReceiveBeginPlay`
  (set `self.startTransform` (`self.GetTransform`)))

(event `self.ReceiveTick`
  (params (DeltaSeconds :type "Float (single-precision)"))
  (set `self.deltaSec` DeltaSeconds)
  (if (`self.cameraTurn`)
    (`self.K2_SetActorTransform` (`KismetMathLibrary.MakeTransform` (`self.K2_GetActorLocation`) (`KismetMathLibrary.MakeRotator` 0.0 0.0 (+ (* (`self.deltaSec`) (`self.speed`)) (.yaw (`self.K2_GetActorRotation`))))))
    (if (`self.CameraClamp`)
      (if (or (<= (.yaw (`self.K2_GetActorRotation`)) (+ (.yaw (.rotation (`self.startTransform`))) (`self.min`))) (>= (.yaw (`self.K2_GetActorRotation`)) (+ (.yaw (.rotation (`self.startTransform`))) (`self.max`))))
        (set `self.speed` (* -1 (`self.speed`)))))))

(event `self.PawnSensing.OnSeePawn`
  (params (Pawn :type "Pawn Object Reference"))
  (bind _asfirst_person_character (cast `/Game/FirstPersonBP/Blueprints/FirstPersonCharacter` Pawn))
  (`/Game/FirstPersonBP/Blueprints/FirstPersonCharacter.respawn` _asfirst_person_character))

(fn `UserConstructionScript`)