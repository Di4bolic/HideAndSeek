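; BP_Valve is a one-shot interactable valve that counts toward opening a linked door.
; On its first Interact, it marks itself active, increments the valve count on MyDoor and calls that door's open check.
; It then swaps the material on its Sphere to show activation, and ignores further interactions.
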(event `self.Interact`
  (bind _mydoor (`self.myDoor`))
  (if (not (`self.isActive`))
    (set `self.isActive` true)
    (set `/Game/NathanBluePrints/DoorValve/BP_DoorValve.numberValve` (+ (`/Game/NathanBluePrints/DoorValve/BP_DoorValve.numberValve` _mydoor) 1) _mydoor)
    (`/Game/NathanBluePrints/DoorValve/BP_DoorValve.checkDoorOpen` (`self.myDoor`))
    (`PrimitiveComponent.SetMaterial` (`self.Sphere`) 0 "/Game/FirstPerson/Meshes/FirstPersonProjectileMaterial.FirstPersonProjectileMaterial")))

(fn `UserConstructionScript`
  (`parent.UserConstructionScript`))