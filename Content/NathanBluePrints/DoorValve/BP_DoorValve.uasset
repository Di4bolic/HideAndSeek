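; BP_DoorValve is a door that opens once enough valves are counted.
; It stores the actor's forward vector at BeginPlay as StartRotation.
; checkDoorOpen compares NumberValve to NumberValveMax, neither changed here, and snaps the Pivot's relative rotation open without animation.
; The 45 is added to the forward vector's Y before conversion back to a rotation, so it is not a 45-degree offset.
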(event `self.ReceiveBeginPlay`
  (set `self.startRotation` (`KismetMathLibrary.Conv_RotatorToVector` (`self.K2_GetActorRotation`))))

(event `checkDoorOpen`
  (if (>= (`self.numberValve`) (`self.numberValveMax`))
    (`SceneComponent.K2_SetRelativeRotation` (`self.pivot`) (`KismetMathLibrary.Conv_VectorToRotator` (+ (`self.startRotation`) (0.0 45.0 0.0))) false false)))

(fn `UserConstructionScript`)