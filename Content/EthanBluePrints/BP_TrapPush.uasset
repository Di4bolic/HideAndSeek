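; BP_TrapPush is a timed water-jet trap that shoves the player along its forward vector with extra upward lift.
; It loops between active and idle via delays from BeginPlay, switching the light red or green and spawning particles and sound while active.
; While active, Tick applies a velocity-change impulse to player 0's FirstPersonCharacter inside EffectZone.
; The construction script sizes and offsets that box from Height.
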(event `self.ReceiveBeginPlay`
  (`self.Activate`))

(event `Activate`
  (bind (_returnvalue_roll _returnvalue_pitch _returnvalue_yaw) (`KismetMathLibrary.BreakRotator` (`SceneComponent.K2_GetComponentRotation` (`self.Cylinder`))))
  (set `self.IsActivated` true)
  (`LightComponent.SetLightColor` (`self.PointLight`) (struct :`R` 1.0 :`A` 1.0) true)
  (bind _returnvalue (`GameplayStatics.SpawnEmitterAtLocation` "/Game/EthanBluePrints/P_Water.P_Water" (`SceneComponent.K2_GetComponentLocation` (`self.Cylinder`)) (`KismetMathLibrary.MakeRotator` _returnvalue_roll _returnvalue_pitch _returnvalue_yaw)))
  (bind _returnvalue_2 (`GameplayStatics.SpawnSoundAtLocation` (`self.SoundToProduce`) (`SceneComponent.K2_GetComponentLocation` (`self.DefaultSceneRoot`)) (struct) 1.0 1.0 0.0 "/Game/EthanBluePrints/SA_ForBasicObjects.SA_ForBasicObjects" null))
  (`AudioComponent.StopDelayed` _returnvalue_2 (`self.ActivationDuration`))
  (`KismetSystemLibrary.Delay` (`self.ActivationDuration`))
  (`self.Desactivate`)
  (`ActorComponent.K2_DestroyComponent` _returnvalue))

(event `Desactivate`
  (set `self.IsActivated` false)
  (`LightComponent.SetLightColor` (`self.PointLight`) (struct :`G` 0.995 :`A` 1.0) true)
  (`KismetSystemLibrary.Delay` (`self.TimeBetweenActivations`))
  (`self.Activate`))

(event `self.ReceiveTick`
  (params (DeltaSeconds :type "Float (single-precision)"))
  (if (`self.IsActivated`)
    (if (`PrimitiveComponent.IsOverlappingActor` (`self.EffectZone`) (`GameplayStatics.GetPlayerPawn` 0))
      (bind _asfirst_person_character (cast `/Game/FirstPersonBP/Blueprints/FirstPersonCharacter` (`GameplayStatics.GetPlayerPawn` 0)))
      (`CharacterMovementComponent.AddImpulse` (`Character.CharacterMovement` _asfirst_person_character) (+ (* (`self.GetActorForwardVector` self) (`self.Power`)) (`KismetMathLibrary.MakeVector` 0.0 0.0 (`self.PowerUp`))) true))))

(fn `UserConstructionScript`
  (bind _height (`self.Height`))
  (`BoxComponent.SetBoxExtent` (`self.EffectZone`) (`KismetMathLibrary.MakeVector` _height 40.0 40.0) true)
  (`SceneComponent.K2_SetRelativeLocation` (`self.EffectZone`) (`KismetMathLibrary.MakeVector` _height) false false))