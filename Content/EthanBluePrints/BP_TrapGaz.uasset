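; Gas trap that emits smoke and sound when interacted with or when the first-person character enters its box zone.
; Each trigger turns the red light green, removes the smoke after a few seconds, then re-arms after a cooldown guarded by IsActive.
; Only overlap raises player fear (AugmentePeur) and fades a HUD smoke overlay in and out through delay loops.
; The construction script sizes and offsets the zone from Height.
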(event `self.ReceiveBeginPlay`
  (set `self.Opacity` 0.0)
  (`LightComponent.SetLightColor` (`self.PointLight`) (struct :`R` 1.0 :`A` 1.0) true))

(event `self.Interact`
  (if (not (`self.IsActive`))
    (set `self.IsActive` true)
    (`LightComponent.SetLightColor` (`self.PointLight`) (struct :`G` 0.995 :`A` 1.0) true)
    (`GameplayStatics.SpawnSoundAtLocation` (`self.SoundToProduce`) (`SceneComponent.K2_GetComponentLocation` (`self.DefaultSceneRoot`)) (struct) 1.0 1.0 0.0 "/Game/EthanBluePrints/SA_ForBasicObjects.SA_ForBasicObjects" null)
    (bind _returnvalue (`GameplayStatics.SpawnEmitterAtLocation` "/Game/StarterContent/Particles/P_Smoke.P_Smoke" (`SceneComponent.K2_GetComponentLocation` (`self.DefaultSceneRoot`))))
    (`KismetSystemLibrary.Delay` 4.0)
    (`ActorComponent.K2_DestroyComponent` _returnvalue)
    (`KismetSystemLibrary.Delay` 10.0)
    (set `self.IsActive` false)
    (`LightComponent.SetLightColor` (`self.PointLight`) (struct :`R` 1.0 :`A` 1.0) true)))

(event `self.EffectZone.OnComponentBeginOverlap`
  (params (OverlappedComponent :type "PrimitiveComponent Object Reference") (OtherActor :type "Actor Object Reference") (OtherComp :type "PrimitiveComponent Object Reference") (OtherBodyIndex :type Integer) (bFromSweep :type Boolean) (SweepResult :type "HitResult Structure (by ref)"))
  (cast `/Game/FirstPersonBP/Blueprints/FirstPersonCharacter` OtherActor)
  (if (not (`self.IsActive`))
    (set `self.IsActive` true)
    (`self.AugmenteOpacity`)
    (`/Game/EthanBluePrints/BP_MyPlayerController.AugmentePeur` (cast `/Game/EthanBluePrints/BP_MyPlayerController` (`GameplayStatics.GetPlayerController` 0) :!pure true) 3)
    (`LightComponent.SetLightColor` (`self.PointLight`) (struct :`G` 0.995 :`A` 1.0) true)
    (`GameplayStatics.SpawnSoundAtLocation` (`self.SoundToProduce`) (`SceneComponent.K2_GetComponentLocation` (`self.DefaultSceneRoot`)) (struct) 1.0 1.0 0.0 "/Game/EthanBluePrints/SA_ForBasicObjects.SA_ForBasicObjects" null)
    (bind _returnvalue (`GameplayStatics.SpawnEmitterAtLocation` "/Game/StarterContent/Particles/P_Smoke.P_Smoke" (`SceneComponent.K2_GetComponentLocation` (`self.DefaultSceneRoot`))))
    (`KismetSystemLibrary.Delay` 4.0)
    (`ActorComponent.K2_DestroyComponent` _returnvalue)
    (`KismetSystemLibrary.Delay` 10.0)
    (set `self.IsActive` false)
    (`LightComponent.SetLightColor` (`self.PointLight`) (struct :`R` 1.0 :`A` 1.0) true)))

(event `AugmenteOpacity`
  (bind _asbp_my_player_controller (cast `/Game/EthanBluePrints/BP_MyPlayerController` (`GameplayStatics.GetPlayerController` 0)))
  (if (< (`self.Opacity`) 1.0) :!label _label
    (bind _output_get (set `self.Opacity` (+ (`self.Opacity`) 0.05)))
    (`Image.SetOpacity` (`/Game/EthanBluePrints/WBP_MyUI.Fume` (`/Game/EthanBluePrints/BP_MyPlayerController.MyUI` _asbp_my_player_controller)) _output_get)
    (`KismetSystemLibrary.Delay` 0.1)
    (goto _label)
    (else
      (`KismetSystemLibrary.Delay` 1.0)
      (if (>= (`self.Opacity`) 0.0) :!label _label_2
        (bind _output_get_2 (set `self.Opacity` (- (`self.Opacity`) 0.05)))
        (`Image.SetOpacity` (`/Game/EthanBluePrints/WBP_MyUI.Fume` (`/Game/EthanBluePrints/BP_MyPlayerController.MyUI` _asbp_my_player_controller)) _output_get_2)
        (`KismetSystemLibrary.Delay` 0.1)
        (goto _label_2)))))

(fn `UserConstructionScript`
  (bind _height (`self.Height`))
  (`BoxComponent.SetBoxExtent` (`self.EffectZone`) (`KismetMathLibrary.MakeVector` _height 40.0 40.0) true)
  (`SceneComponent.K2_SetRelativeLocation` (`self.EffectZone`) (`KismetMathLibrary.MakeVector` _height) false false))