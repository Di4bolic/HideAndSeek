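; BP_TrapStun is a trap actor that stuns the first-person player who steps into it.
; A box overlap fires Triggered, which, while active, plays a sound, raises the controller's fear via AugmentePeur, disables movement and deactivates the trap.
; Movement returns after a TrappedTime delay.
; Interact also deactivates the trap, playing the same sound with attenuation.
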(event `self.Box.OnComponentBeginOverlap`
  (params (OverlappedComponent :type "PrimitiveComponent Object Reference") (OtherActor :type "Actor Object Reference") (OtherComp :type "PrimitiveComponent Object Reference") (OtherBodyIndex :type Integer) (bFromSweep :type Boolean) (SweepResult :type "HitResult Structure (by ref)"))
  (cast `/Game/FirstPersonBP/Blueprints/FirstPersonCharacter` OtherActor)
  (`self.Triggered`))

(event `Triggered`
  (if (`self.IsActive`)
    (`GameplayStatics.SpawnSoundAtLocation` (`self.SoundToProduce`) (`SceneComponent.K2_GetComponentLocation` (`self.DefaultSceneRoot`)) (struct) 1.0 1.0 0.0 null null)
    (bind _asfirst_person_character (cast `/Game/FirstPersonBP/Blueprints/FirstPersonCharacter` (`GameplayStatics.GetPlayerPawn` 0)))
    (`/Game/EthanBluePrints/BP_MyPlayerController.AugmentePeur` (cast `/Game/EthanBluePrints/BP_MyPlayerController` (`GameplayStatics.GetPlayerController` 0) :!pure true) 3)
    (set `/Game/FirstPersonBP/Blueprints/FirstPersonCharacter.canMove` false _asfirst_person_character)
    (set `self.IsActive` false)
    (`KismetSystemLibrary.Delay` (`self.TrappedTime`))
    (set `/Game/FirstPersonBP/Blueprints/FirstPersonCharacter.canMove` true _asfirst_person_character)))

(event `self.Interact`
  (set `self.IsActive` false)
  (`GameplayStatics.SpawnSoundAtLocation` (`self.SoundToProduce`) (`SceneComponent.K2_GetComponentLocation` (`self.DefaultSceneRoot`)) (struct) 1.0 1.0 0.0 "/Game/EthanBluePrints/SA_ForBasicObjects.SA_ForBasicObjects" null))

(fn `UserConstructionScript`
  (`parent.UserConstructionScript`))