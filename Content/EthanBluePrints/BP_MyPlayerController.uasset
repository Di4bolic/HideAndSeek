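; BP_MyPlayerController is the player controller handling interaction, leaving a hidden state, crouching and a fear meter.
; E line-traces from the first-person camera and calls Interact on a hit BP_Interactible.
; While IsHide is set, E instead clears it, teleports the pawn upward and sets CanMove false.
; Left Shift toggles crouch on press and release, while AugmentePeur accumulates fear (Peur) and only prints a message at its maximum.
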(event `Key|E`
  (params (Key :type "Key Structure"))
  (bind _returnvalue (`GameplayStatics.GetPlayerPawn` 0))
  (:`Pressed`
    (if (`self.isHide`)
      (set `self.isHide` false)
      (`self.K2_SetActorLocation` _returnvalue (+ (`self.K2_GetActorLocation` _returnvalue) (0.0 0.0 300.0)) false false)
      (bind _asfirst_person_character (cast `/Game/FirstPersonBP/Blueprints/FirstPersonCharacter` (`GameplayStatics.GetPlayerCharacter` 0)))
      (set `/Game/FirstPersonBP/Blueprints/FirstPersonCharacter.canMove` false _asfirst_person_character)
      (else
        (bind _asfirst_person_character_2 (cast `/Game/FirstPersonBP/Blueprints/FirstPersonCharacter` (`GameplayStatics.GetPlayerPawn` 0)))
        (bind _firstpersoncamera (`/Game/FirstPersonBP/Blueprints/FirstPersonCharacter.FirstPersonCamera` _asfirst_person_character_2))
        (bind _returnvalue_2 (`SceneComponent.K2_GetComponentLocation` _firstpersoncamera))
        (bind _outhit (`KismetSystemLibrary.LineTraceSingle` _returnvalue_2 (+ _returnvalue_2 (* (`SceneComponent.GetForwardVector` _firstpersoncamera) (`self.visibilityDistance`))) "TraceTypeQuery1"))
        (bind _asbp_interactible (cast `/Game/EthanBluePrints/BP_Interactible` (`.HitActor` (`GameplayStatics.BreakHitResult` _outhit))))
        (`/Game/EthanBluePrints/BP_Interactible.Interact` _asbp_interactible)))))

(event `Key|LeftShift`
  (params (Key :type "Key Structure"))
  (:`Pressed`
    (bind _asfirst_person_character (cast `/Game/FirstPersonBP/Blueprints/FirstPersonCharacter` (`GameplayStatics.GetPlayerPawn` 0)))
    (if (`NavMovementComponent.IsCrouching` (`Character.CharacterMovement` _asfirst_person_character)) :!label _label
      (`Character.UnCrouch` _asfirst_person_character)
      (else
        (`Character.Crouch` _asfirst_person_character))))
  (:`Released`
    (goto _label)))

(event `AugmentePeur`
  (params (Augmentation :type Integer))
  (bind _peur (`self.Peur`))
  (set `self.Peur` (+ Augmentation _peur))
  (if (>= _peur (`self.MaxPeur`))
    (`KismetSystemLibrary.PrintString` "Tu as dépassé ta peur max")))

(fn `UserConstructionScript`)